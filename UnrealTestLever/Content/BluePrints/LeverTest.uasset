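; Interactive lever that the player steps up or down between ten positions with left and right mouse clicks while it is touched.
; Each step sends the lever's ID and value to the BP_Pillar found in the level through MovePillarMessage.
; The Pull_UpDown timeline plays or reverses to rotate the handle, stopping itself once its alpha reaches the fraction matching the value.
; OnTouch toggles custom depth on base and handle.
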(event `Key|LeftMouseButton` :consume false
  (params (Key :type "Key Structure"))
  (bind _levervalue (`self.LeverValue`))
  (:`Pressed`
    (if (stale `/Game/BluePrints/Interfaces/BPI_VectorTouch.OnTouch` IsTouching)
      (if (not (== _levervalue 9))
        (set `self.LeverValue` (+ _levervalue 1))
        (set `self.LeverDirection` true)
        (bind _returnvalue (`GameplayStatics.GetActorOfClass` "/Game/BluePrints/BP_Pillar.BP_Pillar_C" :!label _label))
        (message `/Game/BluePrints/Interfaces/BPI_MovePillar.MovePillar` _returnvalue (`self.ID`) (`self.LeverValue`) "Locate")
        (if (stale `Key|RightMouseButton` _output_get)
          (bind (_direction _alpha) (`Timeline|Pull_Up/Down` :!label _label_2)
            (:`Update`
              (`SceneComponent.K2_SetRelativeRotation` (`self.Levier_poignee_low_1`) (`KismetMathLibrary.RLerp` (struct) (struct :`Roll` 120.0) _alpha) false false)
              (if (`self.LeverDirection`)
                (if (>= (/ _alpha 2.0) (/ (`self.LeverValue`) 18.0))
                  (goto _label_2 :!via `Stop`))
                (elif (<= (/ _alpha 2.0) (/ (`self.LeverValue`) 18.0))
                  (goto _label_2 :!via `Stop`)))))
          (else
            (goto _label_2 :!via `Reverse`)))))))

(event `self.ReceiveBeginPlay`
  (`self.EnableInput` (`GameplayStatics.GetPlayerController` 0)))

(event `Key|RightMouseButton` :consume false
  (params (Key :type "Key Structure"))
  (bind _levervalue (`self.LeverValue`))
  (:`Pressed`
    (if (stale `/Game/BluePrints/Interfaces/BPI_VectorTouch.OnTouch` IsTouching)
      (if (not (== _levervalue 0))
        (set `self.LeverValue` (- _levervalue 1))
        (bind _output_get (set `self.LeverDirection` false))
        (goto _label)))))

(event `/Game/BluePrints/Interfaces/BPI_VectorTouch.OnTouch`
  (params (IsTouching :type Boolean))
  (`PrimitiveComponent.SetRenderCustomDepth` (`self.Levier_base_low_1`) IsTouching)
  (`PrimitiveComponent.SetRenderCustomDepth` (`self.Levier_poignee_low_1`) IsTouching))

(fn `UserConstructionScript`)