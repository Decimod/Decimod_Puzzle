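; Lever puzzle control with a rotor and a stick that drive pillar movement, highlighted through custom depth while touched.
; While touched, the mouse wheel steps the rotor through 24 wrapping positions, and left/right clicks step the stick through ten clamped positions.
; Each step messages the BP_Pillar found by GetActorOfClass with ActorID, value and Rotate or ArcRotate.
; Cooldown-gated timelines animate both parts; BeginPlay applies start values to them and the pillar.
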(event `Key|MouseScrollDown`
  (params (Key :type "Key Structure"))
  ; Rotor - Mouse Whell Up/Down - Use For Rotate Pillars
  (:`Pressed`
    (if (stale `/Game/BluePrints/Interfaces/BPI_VectorTouch.OnTouch` IsTouching)
      (if (`self.RotorCooldown`)
        (set `self.RotorCooldown` false)
        (if (== 0 (`self.RotorValue`))
          (set `self.RotorValue` 23)
          (else
            (set `self.RotorValue` (- (`self.RotorValue`) 1))))
        (set `self.RotorEndRotator` (`KismetMathLibrary.MakeRotator` (.roll (`self.RotorStartRotator`)) (.pitch (`self.RotorStartRotator`)) (- (.yaw (`self.RotorStartRotator`)) 15.0)))
        (bind _returnvalue (`GameplayStatics.GetActorOfClass` "/Game/BluePrints/BP_Pillar.BP_Pillar_C" :!label _label))
        (message `/Game/BluePrints/Interfaces/BPI_MovePillar.MovePillar` _returnvalue (`self.ActorID`) (`self.RotorValue`) "Rotate")
        (bind (_direction _alpha) (`Timeline|RotorTimeLine` :!label _label_2)
          (:`Update`
            (`SceneComponent.K2_SetRelativeRotation` (`self.Rotor`) (`KismetMathLibrary.RLerp` (`self.RotorStartRotator`) (`self.RotorEndRotator`) _alpha) false false))
          (:`Finished`
            (set `self.RotorStartRotator` (`self.RotorEndRotator`))
            (set `self.RotorCooldown` true)
            (goto _label_2 :!via `SetNewTime`)))))))

(event `/Game/BluePrints/Interfaces/BPI_VectorTouch.OnTouch`
  (params (IsTouching :type Boolean))
  ; Vector Event - When player look at, Give true and highlight
  (`PrimitiveComponent.SetRenderCustomDepth` (`self.Base`) IsTouching)
  (`PrimitiveComponent.SetRenderCustomDepth` (`self.Rotor`) IsTouching)
  (`PrimitiveComponent.SetRenderCustomDepth` (`self.GizmoLever`) IsTouching)
  (`PrimitiveComponent.SetRenderCustomDepth` (`self.LeverStick`) IsTouching)
  (`PrimitiveComponent.SetRenderCustomDepth` (`self.LeverTop`) IsTouching))

(event `Key|MouseScrollUp`
  (params (Key :type "Key Structure"))
  ; Rotor - Mouse Whell Up/Down - Use For Rotate Pillars
  (:`Pressed`
    (if (stale `/Game/BluePrints/Interfaces/BPI_VectorTouch.OnTouch` IsTouching)
      (if (`self.RotorCooldown`)
        (set `self.RotorCooldown` false)
        (if (== 23 (`self.RotorValue`))
          (set `self.RotorValue` 0)
          (else
            (set `self.RotorValue` (+ (`self.RotorValue`) 1))))
        (set `self.RotorEndRotator` (`KismetMathLibrary.MakeRotator` (.roll (`self.RotorStartRotator`)) (.pitch (`self.RotorStartRotator`)) (+ (.yaw (`self.RotorStartRotator`)) 15.0)))
        (goto _label)))))

(event `self.ReceiveBeginPlay`
  (bind _rotorstartvalue0_23 (`self.RotorStartValue0-23`))
  (bind _leverstartvalue0_9 (`self.LeverStartValue0-9`))
  (`self.EnableInput` (`GameplayStatics.GetPlayerController` 0))
  ; Rotor Initialisation
  (bind _returnvalue (`GameplayStatics.GetActorOfClass` "/Game/BluePrints/BP_Pillar.BP_Pillar_C"))
  (message `/Game/BluePrints/Interfaces/BPI_Init_Pillars.InitPillars` _returnvalue (`self.ActorID`) _rotorstartvalue0_23 "Rotate")
  (set `self.RotorValue` _rotorstartvalue0_23)
  (bind _output_get (set `self.RotorStartRotator` (`KismetMathLibrary.MakeRotator` 0.0 0.0 (`KismetMathLibrary.Conv_IntToDouble` (* 15 _rotorstartvalue0_23)))))
  (`SceneComponent.K2_SetRelativeRotation` (`self.Rotor`) _output_get false false)
  ; Lever Initialisation
  (bind _returnvalue_2 (`GameplayStatics.GetActorOfClass` "/Game/BluePrints/BP_Pillar.BP_Pillar_C"))
  (message `/Game/BluePrints/Interfaces/BPI_Init_Pillars.InitPillars` _returnvalue_2 (`self.ActorID`) _leverstartvalue0_9 "ArcRotate")
  (set `self.LeverValue` _leverstartvalue0_9)
  (set `self.LeverStartRotator` (`KismetMathLibrary.MakeRotator` 0.0 (- (- 100.0 (* _leverstartvalue0_9 11.111111)) 50.0)))
  (`SceneComponent.K2_SetRelativeRotation` (`self.GizmoLever`) (`KismetMathLibrary.MakeRotator` 0.0 (- 50.0 (* (/ 100.0 9.0) _leverstartvalue0_9))) false false))

(event `Key|LeftMouseButton` :consume false
  (params (Key :type "Key Structure"))
  (bind _levervalue (`self.LeverValue`))
  ; Lever - Left/Right Mouse Click - Use For ArcRotate Pillars
  (:`Pressed`
    (if (stale `/Game/BluePrints/Interfaces/BPI_VectorTouch.OnTouch` IsTouching)
      (if (`self.LeverCoolDown`)
        (if (!= _levervalue 9)
          (set `self.LeverValue` (+ _levervalue 1))
          (set `self.LeverCoolDown` false)
          (set `self.LeverEndRotator` (`KismetMathLibrary.MakeRotator` 0.0 (- (.pitch (`self.LeverStartRotator`)) 11.111111)))
          (bind _returnvalue (`GameplayStatics.GetActorOfClass` "/Game/BluePrints/BP_Pillar.BP_Pillar_C" :!label _label_3))
          (message `/Game/BluePrints/Interfaces/BPI_MovePillar.MovePillar` _returnvalue (`self.ActorID`) (`self.LeverValue`) "ArcRotate")
          (bind (_direction _alpha) (`Timeline|Timeline` :!label _label_4)
            (:`Update`
              (`SceneComponent.K2_SetRelativeRotation` (`self.GizmoLever`) (`KismetMathLibrary.RLerp` (`self.LeverStartRotator`) (`self.LeverEndRotator`) _alpha) false false))
            (:`Finished`
              (set `self.LeverStartRotator` (`self.LeverEndRotator`))
              (set `self.LeverCoolDown` true)
              (goto _label_4 :!via `SetNewTime`))))))))

(event `Key|RightMouseButton` :consume false
  (params (Key :type "Key Structure"))
  (bind _levervalue (`self.LeverValue`))
  ; Lever - Left/Right Mouse Click - Use For ArcRotate Pillars
  (:`Pressed`
    (if (stale `/Game/BluePrints/Interfaces/BPI_VectorTouch.OnTouch` IsTouching)
      (if (`self.LeverCoolDown`)
        (if (!= _levervalue 0)
          (set `self.LeverValue` (- _levervalue 1))
          (set `self.LeverCoolDown` false)
          (set `self.LeverEndRotator` (`KismetMathLibrary.MakeRotator` 0.0 (+ (.pitch (`self.LeverStartRotator`)) 11.111111)))
          (goto _label_3))))))

(fn `UserConstructionScript`)