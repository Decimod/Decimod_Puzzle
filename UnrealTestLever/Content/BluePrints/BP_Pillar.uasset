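; BP_Pillar is a pillar actor that slides between two positions in response to a lever value.
; MovePillar checks an ID, then for "Locate" plays or reverses a timeline depending on whether the value rose or fell.
; The timeline lerps the root's relative location and stops once alpha reaches the lever value divided by nine.
; BeginPlay caches the base transform; "Rotate" and "ArcRotate" are recognized but do nothing, while other actions print an error.
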(event `self.ReceiveBeginPlay`
  ; Get Base World Transformation
  (set `self.BaseLocation` (.location (`SceneComponent.GetRelativeTransform` (`self.RootComponent`))))
  (set `self.BaseRotation` (.rotation (`SceneComponent.GetRelativeTransform` (`self.RootComponent`)))))

(event `/Game/BluePrints/Interfaces/BPI_MovePillar.MovePillar`
  (params (ID :type Integer) (LeverValue :type Integer) (Action :type String))
  (bind _lever_value (`self.Lever Value`))
  (if (== ID (`self.ID`))
    (set `self.Lever Value` (`KismetMathLibrary.Conv_IntToDouble` LeverValue))
    (if (`KismetStringLibrary.EqualEqual_StrStr` Action "Locate")
      ; Locate Function - Move the pillar up and down
      (if (> (`self.Lever Value`) (`self.ActualValue`))
        (set `self.PillarDirection` true)
        (set `self.ActualValue` _lever_value)
        (bind (_direction _alpha) (`Timeline|PillarTimeline` :!label _label)
          (:`Update`
            (`SceneComponent.K2_SetRelativeLocation` (`self.RootComponent`) (`KismetMathLibrary.VLerp` (`KismetMathLibrary.MakeVector` (`self.Ax`) (`self.Ay`) (`self.Az`)) (`KismetMathLibrary.MakeVector` (`self.Bx`) (`self.By`) (`self.Bz`)) _alpha) false false)
            (if (`self.PillarDirection`)
              (if (<= (/ (`self.Lever Value`) 9.0) _alpha)
                (goto _label :!via `Stop`))
              (elif (>= (/ (`self.Lever Value`) 9.0) _alpha)
                (goto _label :!via `Stop`)))))
        (else
          (set `self.PillarDirection` false)
          (set `self.ActualValue` _lever_value)
          (goto _label :!via `Reverse`)))
      (elif (`KismetStringLibrary.EqualEqual_StrStr` Action "Rotate")
        _
        (elif (not (`KismetStringLibrary.EqualEqual_StrStr` Action "ArcRotate"))
          (`KismetSystemLibrary.PrintString` "Action Value Error"))))))

(fn `UserConstructionScript`)