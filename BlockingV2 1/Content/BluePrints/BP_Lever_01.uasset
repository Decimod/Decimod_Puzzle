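; Interactable lever that steps a value between 0 and 9 to drive BP_Pillar actors in what looks like a pillar puzzle.
; While touched, it highlights through custom depth, and left or right click raises or lowers the value, rotating the handle on a timeline that gates further input.
; BeginPlay sets the start angle and initializes pillars; each step messages every pillar with the lever's ID and value.
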(event `self.ReceiveBeginPlay`
  (bind _leverstartvalue0_9 (`self.LeverStartValue0-9`))
  (`self.EnableInput` (`GameplayStatics.GetPlayerController` 0))
  ; Set Lever Start Value
  (`KismetSystemLibrary.Delay` 0.2)
  (bind _returnvalue (`GameplayStatics.GetActorOfClass` "/Game/BluePrints/BP_Pillar.BP_Pillar_C"))
  (message `/Game/BluePrints/Interfaces/BPI_Init_Pillars.InitPillars` _returnvalue (`self.ID`) _leverstartvalue0_9 "ArcRotate")
  (set `self.LeverValue` _leverstartvalue0_9)
  (bind _output_get (set `self.LeverStartRotator` (`KismetMathLibrary.MakeRotator` (* _leverstartvalue0_9 13.333333))))
  (`SceneComponent.K2_SetRelativeRotation` (`self.Levier_poignee_low_1`) _output_get false false)
  (bind _outactors (`GameplayStatics.GetAllActorsOfClass` "/Game/BluePrints/BP_Pillar.BP_Pillar_C"))
  (for _array_element _outactors
    (message `/Game/BluePrints/Interfaces/BPI_Init_Pillars.InitPillars` _array_element (`self.ID`) (`self.LeverValue`) "Locate")))

(event `Key|LeftMouseButton` :consume false
  (params (Key :type "Key Structure"))
  (bind _levervalue (`self.LeverValue`))
  ; Lever - Left/Right Mouse Click - Use For ArcRotate Pillars
  (:`Pressed`
    (if (stale `self.OnTouch` IsTouching)
      (if (`self.LeverCoolDown`)
        (if (!= _levervalue 9)
          (set `self.LeverValue` (+ _levervalue 1))
          (set `self.LeverCoolDown` false)
          (set `self.LeverEndRotator` (`KismetMathLibrary.MakeRotator` (+ (.roll (`self.LeverStartRotator`)) 12.0)))
          (bind _outactors (`GameplayStatics.GetAllActorsOfClass` "/Game/BluePrints/BP_Pillar.BP_Pillar_C" :!label _label))
          (for _array_element _outactors
            (message `/Game/BluePrints/Interfaces/BPI_MovePillar.MovePillar` _array_element (`self.ID`) (`self.LeverValue`) "Locate"))
          (bind (_direction _alpha) (`Timeline|Timeline` :!label _label_2)
            (:`Update`
              (`SceneComponent.K2_SetRelativeRotation` (`self.Levier_poignee_low_1`) (`KismetMathLibrary.RLerp` (`self.LeverStartRotator`) (`self.LeverEndRotator`) _alpha) false false))
            (:`Finished`
              (set `self.LeverStartRotator` (`self.LeverEndRotator`))
              (set `self.LeverCoolDown` true)
              (goto _label_2 :!via `SetNewTime`))))))))

(event `self.OnTouch`
  (params (IsTouching :type Boolean))
  ; Vector Event - When player look at, Give true and highlight
  (`PrimitiveComponent.SetRenderCustomDepth` (`self.Levier_base_low_1`) IsTouching)
  (`PrimitiveComponent.SetRenderCustomDepth` (`self.Levier_poignee_low_1`) IsTouching))

(event `Key|RightMouseButton` :consume false
  (params (Key :type "Key Structure"))
  (bind _levervalue (`self.LeverValue`))
  ; Lever - Left/Right Mouse Click - Use For ArcRotate Pillars
  (:`Pressed`
    (if (stale `self.OnTouch` IsTouching)
      (if (`self.LeverCoolDown`)
        (if (!= _levervalue 0)
          (set `self.LeverValue` (- _levervalue 1))
          (set `self.LeverCoolDown` false)
          (set `self.LeverEndRotator` (`KismetMathLibrary.MakeRotator` (- (.roll (`self.LeverStartRotator`)) 12.0)))
          (goto _label))))))

(fn `UserConstructionScript`)