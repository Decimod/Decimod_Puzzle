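; Pillar actor that slides or rotates in response to lever values sent with an ID and an action name.
; InitPillars snaps it to the lever value times an increment for Locate, Rotate (itself) or ArcRotate (its attach parent).
; MovePillar compares against the last lever value to step one increment either way, lerping on a separate timeline per action.
; Rotate also handles lever wrap-around between 23 and 0.
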(event `/Game/BluePrints/Interfaces/BPI_Init_Pillars.InitPillars`
  (params (ID :type Integer) (LeverValue :type Integer) (Action :type String))
  (`KismetSystemLibrary.PrintString` "Init")
  (if (== ID (`self.ID`))
    (if (`KismetStringLibrary.EqualEqual_StrStr` Action "Locate")
      (bind _output_get (set `self.LastLeverLocate` LeverValue))
      (bind _output_get_2 (set `self.StartLocation` (`KismetMathLibrary.MakeVector` (+ (.x (`self.StartLocation`)) (* (.x (`self.LocateIncrement`)) _output_get)) (+ (.y (`self.StartLocation`)) (* (.y (`self.LocateIncrement`)) _output_get)) (+ (.z (`self.StartLocation`)) (* (.z (`self.LocateIncrement`)) _output_get)))))
      (`SceneComponent.K2_SetRelativeLocation` (`self.RootComponent`) _output_get_2 false false)
      (elif (`KismetStringLibrary.EqualEqual_StrStr` Action "Rotate")
        (bind _output_get_3 (set `self.LastLeverRotate` LeverValue))
        (bind _output_get_4 (set `self.StartRotation` (`KismetMathLibrary.MakeRotator` (* (.roll (`self.RotateIncrement`)) _output_get_3) (* (.pitch (`self.RotateIncrement`)) _output_get_3) (* (.yaw (`self.RotateIncrement`)) _output_get_3))))
        (`SceneComponent.K2_SetRelativeRotation` (`self.RootComponent`) _output_get_4 false false)
        (elif (`KismetStringLibrary.EqualEqual_StrStr` Action "ArcRotate")
          (bind _output_get_5 (set `self.LastLeverArcRotate` LeverValue))
          (bind _output_get_6 (set `self.StartArcRotation` (`KismetMathLibrary.MakeRotator` (* (.roll (`self.ArcRotateIncrement`)) _output_get_5) (* (.pitch (`self.ArcRotateIncrement`)) _output_get_5) (* (.yaw (`self.ArcRotateIncrement`)) _output_get_5))))
          (`SceneComponent.K2_SetRelativeRotation` (`SceneComponent.GetAttachParent` (`self.RootComponent`)) _output_get_6 false false)
          (else
            (`KismetSystemLibrary.PrintString` "Action Value Error")))))))

(event `self.ReceiveBeginPlay`
  (set `self.StartLocation` (.location (`SceneComponent.GetRelativeTransform` (`self.RootComponent`))))
  (`KismetSystemLibrary.PrintString` "LocationOK"))

(event `/Game/BluePrints/Interfaces/BPI_MovePillar.MovePillar`
  (params (ID :type Integer) (LeverValue :type Integer) (Action :type String))
  (bind _startlocation (`self.StartLocation`))
  (bind _locateincrement (`self.LocateIncrement`))
  (bind _lastleverrotate (`self.LastLeverRotate`))
  (bind _roll (.roll (`self.StartArcRotation`)))
  (bind _pitch (.pitch (`self.StartArcRotation`)))
  (bind _yaw (.yaw (`self.StartArcRotation`)))
  (bind _roll_2 (.roll (`self.StartRotation`)))
  (bind _pitch_2 (.pitch (`self.StartRotation`)))
  (bind _yaw_2 (.yaw (`self.StartRotation`)))
  (bind _roll_3 (.roll (`self.RotateIncrement`)))
  (bind _pitch_3 (.pitch (`self.RotateIncrement`)))
  (bind _yaw_3 (.yaw (`self.RotateIncrement`)))
  (bind _roll_4 (.roll (`self.ArcRotateIncrement`)))
  (bind _pitch_4 (.pitch (`self.ArcRotateIncrement`)))
  (bind _yaw_4 (.yaw (`self.ArcRotateIncrement`)))
  (if (== ID (`self.ID`))
    (set `self.Lever Value` LeverValue)
    (if (`KismetStringLibrary.EqualEqual_StrStr` Action "Locate")
      ; Locate Function - Move the pillar up and down
      (if (<= (`self.LastLeverLocate`) (`self.Lever Value`))
        (set `self.EndLocation` (+ _startlocation _locateincrement))
        (else
          (set `self.EndLocation` (- _startlocation _locateincrement))))
      (set `self.LastLeverLocate` (`self.Lever Value`))
      (bind (_direction _alpha) (`Timeline|PillarTimeline` :!label _label)
        (:`Update`
          (`SceneComponent.K2_SetRelativeLocation` (`self.RootComponent`) (`KismetMathLibrary.VLerp` (`self.StartLocation`) (`self.EndLocation`) _alpha) false false))
        (:`Finished`
          (set `self.StartLocation` (`self.EndLocation`))
          (goto _label :!via `SetNewTime`)))
      (elif (`KismetStringLibrary.EqualEqual_StrStr` Action "Rotate")
        ; Rotate Function - Rotate the pillar on himself
        (if (== _lastleverrotate 0)
          (if (== (`self.Lever Value`) 23)
            (set `self.LastLeverRotate` 24))
          (elif (== _lastleverrotate 23)
            (if (== (`self.Lever Value`) 0)
              (set `self.LastLeverRotate` -1))))
        (if (<= (`self.LastLeverRotate`) (`self.Lever Value`))
          (set `self.EndRotation` (`KismetMathLibrary.MakeRotator` (+ _roll_2 _roll_3) (+ _pitch_2 _pitch_3) (+ _yaw_2 _yaw_3)))
          (else
            (set `self.EndRotation` (`KismetMathLibrary.MakeRotator` (- _roll_2 _roll_3) (- _pitch_2 _pitch_3) (- _yaw_2 _yaw_3)))))
        (set `self.LastLeverRotate` (`self.Lever Value`))
        (bind (_direction_2 _alpha_2) (`Timeline|Timeline` :!label _label_2)
          (:`Update`
            (`SceneComponent.K2_SetRelativeRotation` (`self.RootComponent`) (`KismetMathLibrary.RLerp` (`self.StartRotation`) (`self.EndRotation`) _alpha_2) false false))
          (:`Finished`
            (set `self.StartRotation` (`self.EndRotation`))
            (goto _label_2 :!via `SetNewTime`)))
        (elif (`KismetStringLibrary.EqualEqual_StrStr` Action "ArcRotate")
          ; Comment
          (if (<= (`self.LastLeverArcRotate`) (`self.Lever Value`))
            (set `self.EndArcRotation` (`KismetMathLibrary.MakeRotator` (+ _roll _roll_4) (+ _pitch _pitch_4) (+ _yaw _yaw_4)))
            (else
              (set `self.EndArcRotation` (`KismetMathLibrary.MakeRotator` (- _roll _roll_4) (- _pitch _pitch_4) (- _yaw _yaw_4)))))
          (set `self.LastLeverArcRotate` (`self.Lever Value`))
          (bind (_direction_3 _alpha_3) (`Timeline|Timeline_0` :!label _label_3)
            (:`Update`
              (`SceneComponent.K2_SetRelativeRotation` (`SceneComponent.GetAttachParent` (`self.RootComponent`)) (`KismetMathLibrary.RLerp` (`self.StartArcRotation`) (`self.EndArcRotation`) _alpha_3) false false))
            (:`Finished`
              (set `self.StartArcRotation` (`self.EndArcRotation`))
              (goto _label_3 :!via `SetNewTime`)))
          (else
            (`KismetSystemLibrary.PrintString` "Action Value Error")))))))

(fn `UserConstructionScript`)